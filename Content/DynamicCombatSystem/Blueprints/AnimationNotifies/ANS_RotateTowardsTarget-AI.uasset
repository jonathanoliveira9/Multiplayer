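; Anim notify state for Dynamic Combat System AI that turns the character toward its target during an animation window.
; On begin, it casts the mesh owner to BP_BaseAI and applies the notify's configurable rotation speed.
; Each tick, it calls the AI's RotateTowardsTarget for a smooth turn toward the blackboard target, and it shows as "RTT" on the timeline.
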(fn GetNotifyName
  (return "RTT"))

(fn ReceivedNotifyBegin
  (params (MeshComp :type Skeletal%20Mesh%20Component%20Object%20Reference) (Animation :type Anim%20Sequence%20Base%20Object%20Reference) (TotalDuration :type Float%20%28single-precision%29))
  ;[1 1 1] Update rotation speed
  (bind _asbp_base_ai (Utilities|Casting|CastToBP_BaseAI (Components|GetOwner MeshComp)))
  (Default|SetRotationSpeed _asbp_base_ai (Variables|Default|GetRotationSpeed))
  (return false))

(fn ReceivedNotifyTick
  (params (MeshComp :type Skeletal%20Mesh%20Component%20Object%20Reference) (Animation :type Anim%20Sequence%20Base%20Object%20Reference) (FrameDeltaTime :type Float%20%28single-precision%29))
  ;[1 1 1] Rotate character smoothly towards blackboard target
  (bind _asbp_base_ai (Utilities|Casting|CastToBP_BaseAI (Components|GetOwner MeshComp)))
  (Default|RotateTowardsTarget _asbp_base_ai)
  (return false))